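; Chunk manager that pre-generates a set number of PCG street megachunks at BeginPlay while showing a loading widget.
; Chunks spawn far below the world one at a time, each PCG completion callback triggering the next spawn and updating the widget.
; Each finished chunk gets an attached BP_ChunkMover carrying its index.
; Once all are built, the widget hides and the first chunk moves to the world origin.
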(event Custom|OnGenerated
  (params (PCGComponent :type PCG%20Component%20Object%20Reference))
  (bind _result (Math|Integer|IncrementInt (Variables|Default|GetGeneratedChunks))
    (:%20%20
      (CallFunction|AddChunkMover _result (Variables|Default|GetCurrentChunk))
      (CallFunction|GenerateChunk)
      (Development|PrintString (Utilities|String|ToString(Text) (Utilities|Text|FormatText "generated chunk #{array index}" _result)))
      (Default|UpdateChunkText (Variables|Default|GetChunkUI) (Variables|Default|GetGeneratedChunks)))))

(event Custom|GenerateChunk
  (if (not (>= (Variables|Default|GetGeneratedChunks) (Variables|Default|GetChunkAmount)))
    (bind _returnvalue (Game|SpawnActorfromClass :Class "/Game/Blueprints/Chunk/BP_Megachunk.BP_Megachunk_C" :SpawnTransform (Math|Transform|MakeTransform (Math|Vector|MakeVector 0.0 0.0 -99999999.0) "0, 0, 0" "1.000000,1.000000,1.000000") :CollisionHandlingOverride "Undefined" :TransformScaleMethod "MultiplyWithRoot" :WorldParametersReference "/Game/DataAssets/DA_WorldParameters.DA_WorldParameters" :SpawnedSpecialActor 0 :Instigator 0))
    (Variables|Default|SetCurrentChunk _returnvalue)
    (Utilities|Array|Add (Variables|Default|GetMegaChunks) _returnvalue)
    (PCG|Generate (Variables|/Script/ProjectMomentum.Megachunk|GetPCG_Street _returnvalue) false)
    (EventDispatchers|AssignOnPCGGraphGeneratedExternal (Variables|/Script/ProjectMomentum.Megachunk|GetPCG_Street _returnvalue) (delegate Custom|OnGenerated))
    (else
      (Development|PrintString (Utilities|String|ToString(Text) (Utilities|Text|FormatText "All {Total Chunks} chunks spawned" (Variables|Default|GetChunkAmount))))
      (Widget|SetVisibility (Variables|Default|GetChunkUI) "Hidden")
      (Transformation|SetActorLocation (Utilities|Array|Get(acopy) (Variables|Default|GetMegaChunks)) "0, 0, 0" false false))))

(event Custom|AddChunkMover
  (params (Index :type Integer) (Parent :type Actor%20Object%20Reference))
  (bind _returnvalue (Game|SpawnActorfromClass "/Game/Blueprints/Chunk/BP_ChunkMover.BP_ChunkMover_C" (Math|Transform|MakeTransform "0.0,0.0,0.0" "0, 0, 0" "1.000000,1.000000,1.000000") "Undefined" "MultiplyWithRoot" 0 Index 0))
  (Transformation|AttachActorToActor _returnvalue Parent "None" "KeepRelative" "KeepRelative" "KeepRelative" true))

(event EventBeginPlay
  (Variables|Default|SetbIsSpawning true)
  (CallFunction|GenerateChunk)
  (bind _returnvalue (UserInterface|CreateWidget "/Game/Blueprints/UI/WBP_ChunkLoading.WBP_ChunkLoading_C" (Game|GetPlayerController 0)))
  (bind _output_get (Variables|Default|SetChunkUI _returnvalue))
  (Variables|/Game/Blueprints/UI/WBP_ChunkLoading.WBP_ChunkLoading_C|SetTotalChunks _output_get (Variables|Default|GetChunkAmount))
  (UserInterface|Viewport|AddtoViewport _output_get 0))

(fn ConstructionScript)