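; BP_ChunkMover is a chunk-recycling actor for what looks like an endlessly repeating level, but most of its logic is disconnected.
; BeginPlay, overlap and RandomChunk are empty, leaving unwired nodes for finding BP_ChunkManager, detecting the player and recursively picking another random MegaChunk.
; ResetDoOnce only resets a DoOnce gate.
; That gate's unreachable output would teleport the chosen chunk ahead along Y and update the manager's chunk list.
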(event Custom|RandomChunk)

(event Custom|ResetDoOnce
  (bind _chunkmanager (Variables|Default|GetChunkManager))
  (Utilities|FlowControl|DoOnce false) ; enters at Reset
)

(event EventBeginPlay)

(event Collision|EventActorBeginOverlap
  (params (OtherActor :type Actor%20Object%20Reference)))

(fn ConstructionScript)