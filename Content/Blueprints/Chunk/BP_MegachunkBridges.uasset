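; BP_MegachunkBridges is a chunk Blueprint that triggers procedural bridge, facade or street generation on BeginPlay.
; Nested thresholds on ChunkChoiceValue select one PCG component, and one band between facades and streets generates nothing.
; Each active branch writes a random ChunkSeed into a PCG graph instance, then calls Generate.
; The bridge branch seeds PCGNewBridges' graph but generates PCGBridges.
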(event EventBeginPlay
  (if (> (Variables|Default|GetChunkChoiceValue) 2.5)
    (if (> (Variables|Default|GetChunkChoiceValue) 5.0)
      (if (> (Variables|Default|GetChunkChoiceValue) 7.5)
        (bind _output_get (Variables|Default|SetPCGStreetGraph (Variables|/Script/PCG.PCGComponent|GetGraphInstance (Variables|Default|GetPCG_Street))))
        (bind _output_get_2 (Variables|Default|SetChunkSeed (Math|Random|RandomIntegerinRange 0 1024)))
        (Class|PCGGraphParametersHelpers|SetInt32Parameter _output_get "ChunkSeed" _output_get_2)
        (PCG|Generate (Variables|Default|GetPCG_Street) false))
      (else
        (bind _output_get_3 (Variables|Default|SetPCGFacadeGraph (Variables|/Script/PCG.PCGComponent|GetGraphInstance (Variables|Default|GetPCG_Facades))))
        (bind _output_get_4 (Variables|Default|SetChunkSeed (Math|Random|RandomIntegerinRange 0 1024)))
        (Class|PCGGraphParametersHelpers|SetInt32Parameter _output_get_3 "ChunkSeed" _output_get_4)
        (PCG|Generate (Variables|Default|GetPCG_Facades) false)))
    (else
      (bind _output_get_5 (Variables|Default|SetPCGBridgesGraph (Variables|/Script/PCG.PCGComponent|GetGraphInstance (Variables|Default|GetPCG%20NewBridges))))
      (bind _output_get_6 (Variables|Default|SetChunkSeed (Math|Random|RandomIntegerinRange 0 1024)))
      (Class|PCGGraphParametersHelpers|SetInt32Parameter _output_get_5 "ChunkSeed" _output_get_6)
      (PCG|Generate (Variables|Default|GetPCG_Bridges) false))))

(fn ConstructionScript)