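; Megachunk actor that procedurally builds a seeded corridor chunk of street, facades and bridges through PCG.
; FinalizeonGameThread places the actor, then rolls corridor width, height and ledge spacing from world parameter ranges.
; Three PCG components generate in sequence, each completion callback configuring and starting the next.
; Construction script sets the HISM components to BlockAll; the bridge-completion handler and CollectWebAnchors are empty stubs.
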(event Custom|OnStreetGenerated
  (params (PCGComponent :type PCG%20Component%20Object%20Reference))
  ;[0.15 0.15 0.15 0.5] Set Facade Parameters
  (bind _output_get (Variables|Default|SetPCGFacadeGraph (Variables|/Script/PCG.PCGComponent|GetGraphInstance (Variables|Default|GetPCG_Facades))))
  (Effects|Components|ParticleSystem|SetFloatParameter _output_get "LedgeSpacing" (Variables|Default|GetChunkLedgeSpacing))
  (Effects|Components|ParticleSystem|SetFloatParameter (Variables|Default|GetPCGFacadeGraph) "ProtrusionChance" (Variables|/Script/ProjectMomentum.DA_WorldParameters|GetProtrusionChance (Variables|Default|GetWorldParametersReference)))
  (Effects|Components|ParticleSystem|SetFloatParameter (Variables|Default|GetPCGFacadeGraph) "BuildingDepthMin" (Variables|/Script/ProjectMomentum.DA_WorldParameters|GetBuildingDepthMin (Variables|Default|GetWorldParametersReference)))
  (Effects|Components|ParticleSystem|SetFloatParameter (Variables|Default|GetPCGFacadeGraph) "BuildingDepthMax" (Variables|/Script/ProjectMomentum.DA_WorldParameters|GetBuildingDepthMax (Variables|Default|GetWorldParametersReference)))
  (Effects|Components|ParticleSystem|SetFloatParameter (Variables|Default|GetPCGFacadeGraph) "CorridorWidth" (Variables|Default|GetChunkCorridorWidth))
  (Effects|Components|ParticleSystem|SetFloatParameter (Variables|Default|GetPCGFacadeGraph) "CorridorHeight" (Variables|Default|GetChunkCorridorHeight))
  (Class|PCGGraphParametersHelpers|SetInt64Parameter (Variables|Default|GetPCGFacadeGraph) "ChunkSeed" (Class|KismetMathLibrary|ToInt64(Integer) (Variables|Default|GetChunkSeed)))
  (EventDispatchers|BindEventtoOnPCGGraphGeneratedExternal (Variables|Default|GetPCG_Facades) (delegate Custom|OnFacadesGenerated))
  (PCG|Generate (Variables|Default|GetPCG_Facades) false))

(event Custom|OnFacadesGenerated
  (params (PCGComponent :type PCG%20Component%20Object%20Reference))
  ;[0.15 0.15 0.15 0.5] Set Bridge Parameters
  (bind _output_get (Variables|Default|SetPCGBridgesGraph (Variables|/Script/PCG.PCGComponent|GetGraphInstance (Variables|Default|GetPCG_Bridges))))
  (Class|PCGGraphParametersHelpers|SetInt32Parameter _output_get "BridgeCountMin" (Variables|/Script/ProjectMomentum.DA_WorldParameters|GetBridgeCountMin (Variables|Default|GetWorldParametersReference)))
  (Class|PCGGraphParametersHelpers|SetInt32Parameter (Variables|Default|GetPCGBridgesGraph) "BridgeCountMax" (Variables|/Script/ProjectMomentum.DA_WorldParameters|GetBridgeCountMax (Variables|Default|GetWorldParametersReference)))
  (Effects|Components|ParticleSystem|SetFloatParameter (Variables|Default|GetPCGBridgesGraph) "BridgeSpanMax" 0.0)
  (Effects|Components|ParticleSystem|SetFloatParameter (Variables|Default|GetPCGBridgesGraph) "PierSpacing" 0.0)
  (EventDispatchers|BindEventtoOnPCGGraphGeneratedExternal (Variables|Default|GetPCG_Bridges) (delegate Custom|OnBridgesGenerated))
  (PCG|Generate (Variables|Default|GetPCG_Bridges) false))

(event Custom|OnBridgesGenerated
  (params (PCGComponent :type PCG%20Component%20Object%20Reference)))

(event EventFinalizeonGameThread
  ;[0.15 0.15 0.15 0.5] FinalizeOnGameThread // Set Street Parameters
  (Rendering|SetActorHiddenInGame false)
  (Transformation|SetActorLocation (Variables|Default|GetChunkOrigin) false false)
  (Variables|Default|SetChunkRandomStream (Math|Random|MakeRandomStream (.initialseed (Math|Random|MakeRandomStream (Variables|Default|GetChunkSeed)))))
  (CallFunction|ResolveChunkParameters)
  (bind _output_get (Variables|Default|SetPCGStreetGraph (Variables|/Script/PCG.PCGComponent|GetGraphInstance (Variables|Default|GetPCG_Street))))
  (Effects|Components|ParticleSystem|SetFloatParameter _output_get "CorridorWidth" (Variables|Default|GetChunkCorridorWidth))
  (Effects|Components|ParticleSystem|SetFloatParameter (Variables|Default|GetPCGStreetGraph) "CorridorHeight" (Variables|Default|GetChunkCorridorHeight))
  (Effects|Components|ParticleSystem|SetFloatParameter (Variables|Default|GetPCGStreetGraph) "None" (Variables|/Script/ProjectMomentum.DA_WorldParameters|GetChunkLength (Variables|Default|GetWorldParametersReference)))
  (Class|PCGGraphParametersHelpers|SetInt64Parameter (Variables|Default|GetPCGStreetGraph) "None" (Class|KismetMathLibrary|ToInt64(Integer) (Variables|Default|GetChunkSeed)))
  (EventDispatchers|AssignOnPCGGraphGeneratedExternal (Variables|Default|GetPCG_Street) (delegate Custom|OnStreetGenerated))
  (PCG|Generate (Variables|Default|GetPCG_Street) false))

(fn ConstructionScript
  (Collision|SetCollisionProfileName (Variables|Default|GetHISM_Floor) "BlockAll" true :!class /Script/Engine.PrimitiveComponent))

(fn ResolveChunkParameters
  (bind _worldparametersreference (Variables|Default|GetWorldParametersReference))
  (bind _worldparametersreference_2 (Variables|Default|GetWorldParametersReference))
  (bind _worldparametersreference_3 (Variables|Default|GetWorldParametersReference))
  (Variables|Default|SetChunkCorridorWidth (Math|Random|RandomFloatinRangefromStream (Variables|Default|GetChunkRandomStream) (Variables|/Script/ProjectMomentum.DA_WorldParameters|GetCorridorWidthMin _worldparametersreference_2) (Variables|/Script/ProjectMomentum.DA_WorldParameters|GetCorridorWidthMax _worldparametersreference_2)))
  (Variables|Default|SetChunkCorridorHeight (Math|Random|RandomFloatinRangefromStream (Variables|Default|GetChunkRandomStream) (Variables|/Script/ProjectMomentum.DA_WorldParameters|GetCorridorHeightMin _worldparametersreference_3) (Variables|/Script/ProjectMomentum.DA_WorldParameters|GetCorridorHeightMax _worldparametersreference_3)))
  (Variables|Default|SetChunkLedgeSpacing (Math|Random|RandomFloatinRangefromStream (Variables|Default|GetChunkRandomStream) (Variables|/Script/ProjectMomentum.DA_WorldParameters|GetLedgeSpacingMin _worldparametersreference) (Variables|/Script/ProjectMomentum.DA_WorldParameters|GetLedgeSpacingMax _worldparametersreference))))

(fn CollectWebAnchors)