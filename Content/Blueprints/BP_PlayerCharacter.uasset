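; Player character with web-swing traversal: Fire traces from the camera and sends a cable to the trace location, and Left Shift boosts gravity to dive.
; Tick drives web travel, swinging and reel-back through boolean states.
; Swinging simulates physics on the capsule, steers with input forces, and enforces rope length by clamping position and removing outward velocity.
; Releasing Fire restores falling movement, launches with the physics velocity and starts reel-back.
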(event Custom|FireWeb
  (bind _camera (Variables|Default|GetCamera))
  (bind _returnvalue (Transformation|GetWorldLocation _camera))
  ;[0.15 0.15 0.15 0.5] Fire The Web
  (bind _outhit (Collision|LineTraceByChannel _returnvalue (+ _returnvalue (* (Math|Vector|GetForwardVector _camera) 5e+03)) "TraceTypeQuery1" false 0 "None"))
  (bind _output_get (Variables|Default|SetWebHitLocation (.location _outhit)))
  (Variables|Default|SetWebLength (Math|Vector|Distance(Vector) _output_get (Transformation|GetActorLocation)))
  (Variables|Default|SetbWebFired true)
  (Development|PrintString "HitValid" true true "(R=0.000000,G=1.000000,B=0.125761,A=1.000000)")
  (Variables|Default|SetWebStart (Transformation|GetActorLocation))
  (Rendering|SetVisibility (Variables|Default|GetRopeSwing) true false)
  (Transformation|SetWorldLocation (Variables|Default|GetWebAttachPoint) (Variables|Default|GetWebHitLocation) false false))

(event Custom|RemoveWeb
  ;[0.15 0.15 0.15 0.5] RemoveWeb
  (Development|PrintString "IsReeling")
  (bind _returnvalue (Physics|GetPhysicsLinearVelocity (Variables|Default|GetCapsuleComponent) "None"))
  (Variables|Default|SetLaunchVelocity _returnvalue)
  (Physics|SetSimulatePhysics (Variables|Default|GetCapsuleComponent) false)
  (Pawn|Components|CharacterMovement|SetMovementMode (Variables|Character|GetCharacterMovement) "MOVE_Falling" 0)
  (Character|LaunchCharacter (Variables|Default|GetLaunchVelocity) true true)
  (Variables|Default|SetbIsSwinging false)
  (Variables|Default|SetbIsReeling true))

(event Custom|AttachRope
  (bind _capsulecomponent (Variables|Default|GetCapsuleComponent))
  ;[0.15 0.15 0.15 0.5] AttachRope
  (Variables|Default|SetbIsSwinging true)
  (Physics|SetSimulatePhysics _capsulecomponent true)
  (Class|PrimitiveComponent|SetLinearDamping _capsulecomponent 0.05)
  (Pawn|Components|CharacterMovement|SetMovementMode (Variables|Character|GetCharacterMovement) "MOVE_Flying" 0)
  (Variables|/Script/CableComponent.CableComponent|SetEndLocation (Variables|Default|GetRopeSwing) (Utilities|WorldtoLocalSpace (Variables|Default|GetWebHitLocation)))
  (bind _output_get (Variables|Default|SetWebLength (Math|Vector|Distance(Vector) (Transformation|GetActorLocation) (Variables|Default|GetWebHitLocation))))
  (Variables|/Script/CableComponent.CableComponent|SetCableLength (Variables|Default|GetRopeSwing) _output_get)
  (Transformation|SetWorldLocation (Variables|Default|GetWebAttachPoint) (Variables|Default|GetWebHitLocation) false false))

(event Input|EnhancedActionEvents|EnhancedInputActionIA_Fire
  (params (ActionValue :type Boolean) (ElapsedSeconds :type Float%20%28double-precision%29) (TriggeredSeconds :type Float%20%28double-precision%29) (InputAction :type Input%20Action%20Object%20Reference :default "/Game/Inputs/IA_Fire.IA_Fire"))
  ;[0.15 0.15 0.15 0.5] Fire Button
  (:Triggered
    (if (not (Variables|Default|GetbWebFired))
      (CallFunction|FireWeb)))
  (:Canceled
    (if (Variables|Default|GetbWebFired) :!label _label
      (CallFunction|RemoveWeb)))
  (:Completed
    (goto _label)))

(event Input|EnhancedActionEvents|EnhancedInputActionIA_Move
  (params (ActionValue :type Vector%202D%20Structure) (ElapsedSeconds :type Float%20%28double-precision%29) (TriggeredSeconds :type Float%20%28double-precision%29) (InputAction :type Input%20Action%20Object%20Reference :default "/Game/Inputs/IA_Move.IA_Move"))
  ;[0.15 0.15 0.15 0.5] Move Input
  (if (Variables|Default|GetbIsSwinging)
    (Variables|Default|SetSwingInputX (.x ActionValue))
    (Variables|Default|SetSwingInputY (.y ActionValue))))

(event EventBeginPlay
  ;[0.15 0.15 0.15 0.5] BeginPlay
  (bind _returnvalue (UserInterface|CreateWidget "/Game/Blueprints/WBP_UI.WBP_UI_C"))
  (UserInterface|Viewport|AddtoViewport _returnvalue 0)
  (Rendering|SetVisibility (Variables|Default|GetRopeSwing) false false)
  (Variables|Default|SetGravity%20Scale (Variables|/Script/Engine.CharacterMovementComponent|GetGravityScale (Variables|Character|GetCharacterMovement)))
  (Variables|Default|SetBaseFOV (Variables|/Script/Engine.CameraComponent|GetFieldOfView (Variables|Default|GetCamera))))

(event EventTick
  (params (DeltaSeconds :type Float%20%28single-precision%29))
  ;[0.15 0.15 0.15 0.5] Tick
  (Utilities|FlowControl|Sequence
    (:then_0
      (Camera|SetFieldOfView (Variables|Default|GetCamera) (Math|Float|Clamp(Float) (* (+ (Variables|/Script/Engine.CameraComponent|GetFieldOfView (Variables|Default|GetCamera)) 0.0) 0.1) (Variables|Default|GetBaseFOV) (Variables|Default|GetMaxFOV))))
    (:then_1
      (if (not (Variables|Default|GetbIsReeling))
        (if (and (Variables|Default|GetbWebFired) (not (Variables|Default|GetbIsSwinging)))
          (CallFunction|AttachedButNoSwing DeltaSeconds)
          (elif (and (Variables|Default|GetbWebFired) (Variables|Default|GetbIsSwinging))
            (Utilities|FlowControl|Sequence
              (:then_0
                (CallFunction|Swinging))
              (:then_1
                (Utilities|FlowControl|Delay 0.1)
                (CallFunction|RopeSolidity)))))
        (else
          (CallFunction|ReelBack DeltaSeconds))))))

(event Input|KeyboardEvents|LeftShift
  (params (Key :type Key%20Structure :default "None"))
  ;[0.15 0.15 0.15 0.5] Dive
  (:Pressed
    (Variables|/Script/Engine.CharacterMovementComponent|SetGravityScale (Variables|Character|GetCharacterMovement) (Variables|Default|GetBoostedGravity)))
  (:Released
    (Variables|/Script/Engine.CharacterMovementComponent|SetGravityScale (Variables|Character|GetCharacterMovement) (Variables|Default|GetGravity%20Scale))))

(fn ConstructionScript)

(fn AttachedButNoSwing
  (params (A :type Float%20%28double-precision%29))
  (bind _output_get (Variables|Default|SetWebTravelProgress (+ (Variables|Default|GetWebTravelProgress) (* A (Variables|Default|GetRopeTravelSpeed)))))
  (Transformation|SetWorldLocation (Variables|Default|GetWebAttachPoint) (Math|Vector|Lerp(Vector) (Transformation|GetActorLocation) (Variables|Default|GetWebHitLocation) (Math|Float|Clamp(Float) _output_get)) false false)
  (bind _output_get_2 (Variables|/Script/CableComponent.CableComponent|SetEndLocation (Variables|Default|GetRopeSwing) (Utilities|WorldtoLocalSpace (Math|Vector|Lerp(Vector) (Transformation|GetActorLocation) (Variables|Default|GetWebHitLocation) (Math|Float|Clamp(Float) _output_get)))))
  (Variables|/Script/CableComponent.CableComponent|SetCableLength (Variables|Default|GetRopeSwing) (Math|Vector|Distance(Vector) _output_get_2 (Transformation|GetActorLocation)))
  (if (>= (Variables|Default|GetWebTravelProgress) 1.0)
    (CallFunction|AttachRope)))

(fn Swinging
  (bind _returnvalue (Pawn|GetControlRotation :!class /Script/Engine.Pawn))
  (bind _returnvalue_2 (Transformation|GetActorLocation))
  (bind _webhitlocation (Variables|Default|GetWebHitLocation))
  (bind _ropeswing (Variables|Default|GetRopeSwing))
  (bind _returnvalue_3 (- _returnvalue_2 _webhitlocation))
  (bind _returnvalue_4 (Math|Vector|Normalize _returnvalue_3))
  (if (not (Variables|Default|GetbBoosted))
    (Physics|AddForce (Variables|Default|GetCapsuleComponent) (* (+ (* (Math|Vector|GetForwardVector _returnvalue) (Variables|Default|GetSwingInputY)) (* (Math|Vector|GetRightVector _returnvalue) (Variables|Default|GetSwingInputX))) 5e+02) "None" true)
    (Variables|/Script/CableComponent.CableComponent|SetEndLocation _ropeswing (Utilities|WorldtoLocalSpace (Variables|Default|GetWebHitLocation)))
    (Variables|/Script/CableComponent.CableComponent|SetCableLength _ropeswing (Variables|Default|GetWebLength))
    (if (> (Math|Vector|VectorLength _returnvalue_3) (Variables|Default|GetWebLength))
      (Transformation|SetActorLocation (+ (Variables|Default|GetWebHitLocation) (* _returnvalue_4 (Variables|Default|GetWebLength))) false false)
      (bind _returnvalue_5 (Physics|GetPhysicsLinearVelocity (Variables|Default|GetCapsuleComponent) "None"))
      (if (> (Math|Vector|DotProduct _returnvalue_5 _returnvalue_4) 0.0)
        (Physics|SetPhysicsLinearVelocity (Variables|Default|GetCapsuleComponent) (- _returnvalue_5 (* _returnvalue_4 (Math|Vector|DotProduct _returnvalue_5 _returnvalue_4))) false "None")))))

(fn RopeSolidity
  (bind _returnvalue (Pawn|GetController))
  (bind _returnvalue_2 (Pawn|GetControlRotation _returnvalue :!class /Script/Engine.Controller))
  (bind _returnvalue_3 (Math|Rotator|MakeRotator (.yaw _returnvalue_2) 0.0 0.0))
  (Physics|AddForce (Variables|Default|GetCapsuleComponent) (* (+ (* (Math|Vector|GetForwardVector _returnvalue_3) (Variables|Default|GetSwingInputY)) (* (Math|Vector|GetRightVector _returnvalue_3) (Variables|Default|GetSwingInputX))) (Variables|Default|GetAirControlForce)) "None" false))

(fn ReelBack
  (params (A :type Float%20%28double-precision%29))
  (bind _returnvalue (Transformation|GetActorLocation))
  (bind _ropeswing (Variables|Default|GetRopeSwing))
  (bind _output_get (Variables|Default|SetReelProgress (+ (Variables|Default|GetReelProgress) (* A (Variables|Default|GetReelTravelSpeed)))))
  (Development|PrintString "Reeling")
  (bind _output_get_2 (Variables|/Script/CableComponent.CableComponent|SetEndLocation _ropeswing (Utilities|WorldtoLocalSpace (Math|Vector|Lerp(Vector) (Variables|Default|GetWebHitLocation) _returnvalue (Math|Float|Clamp(Float) _output_get)))))
  (Variables|/Script/CableComponent.CableComponent|SetCableLength _ropeswing (Math|Vector|Distance(Vector) _output_get_2 _returnvalue))
  (if (>= (Variables|Default|GetReelProgress) 0.0)
    (Variables|Default|SetbIsReeling false)
    (Variables|Default|SetbWebFired false)
    (Variables|Default|SetWebTravelProgress 0.0)
    (Variables|Default|SetReelProgress 0.0)
    (Rendering|SetVisibility (Variables|Default|GetRopeSwing) false false)))